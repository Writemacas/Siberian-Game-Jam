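; Player controller that turns input into movement, camera, pause menu, element switching, elemental skill and bow actions, relaying the latter ones through Call events.
; Holding FocusToWisp sets the shield-aim camera and opens a Tick-fed gate that keeps control rotation on the WispChar found at BeginPlay.
; Aiming and skill flags block conflicting actions, and aiming halves look speed.
; Wind, ice and fire switches share a delayed DoOnce cooldown, with wind selected on first Tick.
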(event EventBeginPlay
  ;[0.4001 1 0.288] Фокусировка на актере-огоньке
  (bind _returnvalue (Actor|GetActorOfClass "/Game/CodeFolder/Blueprints/Ai_Logic/Wisp/WispChar.WispChar_C"))
  (if (Utilities|IsValid _returnvalue)
    (bind _asthird_person_character (Utilities|Casting|CastToThirdPersonCharacter (Pawn|GetControlledPawn)))
    (Utilities|FlowControl|Sequence
      (:then_0
        (Utilities|FlowControl|Gate true) ; enters at Open
      )
      (:then_1
        (Utilities|FlowControl|Gate true) ; enters at Open
      ))))

(event EventTick
  (params (DeltaSeconds :type Float%20%28single-precision%29))
  ;[1 0.04683 0] ПОКА НЕ ПРИДУМАНО ДРУГОГО РЕШЕНИЯ
  (Utilities|FlowControl|Sequence
    (:then_0
      ;[0.4001 1 0.288] Фокусировка на актере-огоньке
      (Utilities|FlowControl|Gate true
        (:Exit
          (Pawn|SetControlRotation (Math|Rotator|MakeRotator (.roll (Math|Rotator|FindLookatRotation (Transformation|GetActorLocation (stale EventBeginPlay _asthird_person_character)) (Transformation|GetWorldLocation (Variables|/Game/CodeFolder/Blueprints/Ai_Logic/Wisp/WispChar.WispChar_C|GetShell (stale EventBeginPlay _returnvalue))))) (+ 1e+01 (.pitch (Math|Rotator|FindLookatRotation (Transformation|GetActorLocation (stale EventBeginPlay _asthird_person_character)) (Transformation|GetWorldLocation (Variables|/Game/CodeFolder/Blueprints/Ai_Logic/Wisp/WispChar.WispChar_C|GetShell (stale EventBeginPlay _returnvalue)))))) (.yaw (Math|Rotator|FindLookatRotation (Transformation|GetActorLocation (stale EventBeginPlay _asthird_person_character)) (Transformation|GetWorldLocation (Variables|/Game/CodeFolder/Blueprints/Ai_Logic/Wisp/WispChar.WispChar_C|GetShell (stale EventBeginPlay _returnvalue))))))))))
    (:then_1
      (Utilities|FlowControl|DoOnce false
        (:Completed
          ;[0 1 0.06815] Смена стихий
          (Variables|Default|SetElementNumber 0)
          (Utilities|FlowControl|DoOnce false :!label _label
            (:Completed
              (Default|CallSwithElement (Variables|Default|GetElementNumber))
              (Utilities|FlowControl|Delay (Variables|Default|GetSwithElementDelay))
              (goto _label Reset))))))))

(event Input|ActionEvents|InputActionMenuEsc
  (params (Key :type Key%20Structure :default "None"))
  ;[0 1 0.03834] Вызов меню паузы по нажатию Esc
  (:Pressed
    (Default|CallShowMenuUi)
    (Variables|Default|SetbShowMouseCursor true)))

(event Input|ActionEvents|InputActionSwithToWind
  (params (Key :type Key%20Structure :default "None"))
  ;[0 1 0.06815] Смена стихий
  (:Pressed
    (if (not (Variables|Default|GetIsAiming))
      (if (not (Variables|Default|GetIsElementalSkill))
        (Variables|Default|SetElementNumber 0)
        (Utilities|FlowControl|DoOnce false :!label _label
          (:Completed
            (Default|CallSwithElement (Variables|Default|GetElementNumber))
            (Utilities|FlowControl|Delay (Variables|Default|GetSwithElementDelay))
            (goto _label Reset)))))))

(event Input|ActionEvents|InputActionSwithToIce
  (params (Key :type Key%20Structure :default "None"))
  ;[0 1 0.06815] Смена стихий
  (:Pressed
    (if (not (Variables|Default|GetIsAiming))
      (if (not (Variables|Default|GetIsElementalSkill))
        (Variables|Default|SetElementNumber 1)
        (Utilities|FlowControl|DoOnce false :!label _label
          (:Completed
            (Default|CallSwithElement (Variables|Default|GetElementNumber))
            (Utilities|FlowControl|Delay (Variables|Default|GetSwithElementDelay))
            (goto _label Reset)))))))

(event Input|ActionEvents|InputActionSwithToFire
  (params (Key :type Key%20Structure :default "None"))
  ;[0 1 0.06815] Смена стихий
  (:Pressed
    (if (not (Variables|Default|GetIsAiming))
      (if (not (Variables|Default|GetIsElementalSkill))
        (Variables|Default|SetElementNumber 2)
        (Utilities|FlowControl|DoOnce false :!label _label
          (:Completed
            (Default|CallSwithElement (Variables|Default|GetElementNumber))
            (Utilities|FlowControl|Delay (Variables|Default|GetSwithElementDelay))
            (goto _label Reset)))))))

(event Input|ActionEvents|InputActionAttackBow
  (params (Key :type Key%20Structure :default "None"))
  ;[1 0.8557 0] Умения, атака копьем+счетчик комбо, стрельба из лука
  (:Pressed
    (Variables|Default|SetIsAiming true)
    (if (not (Variables|Default|GetIsElementalSkill)) :!label _label
      (Default|CallSwithAimMode (Variables|Default|GetElementNumber))))
  (:Released
    (Variables|Default|SetIsAiming false)
    (goto _label)))

(event Input|ActionEvents|InputActionElementalSkill
  (params (Key :type Key%20Structure :default "None"))
  ;[1 0.8557 0] Умения, атака копьем+счетчик комбо, стрельба из лука
  (:Pressed
    (Variables|Default|SetIsElementalSkill true)
    (if (not (Variables|Default|GetIsAiming)) :!label _label
      (Default|CallElementalUse (Variables|Default|GetElementNumber))))
  (:Released
    (Variables|Default|SetIsElementalSkill false)
    (goto _label)))

(event Input|ActionEvents|InputActionAttack
  (params (Key :type Key%20Structure :default "None"))
  (bind _isaiming (Variables|Default|GetIsAiming))
  ;[1 0.8557 0] Умения, атака копьем+счетчик комбо, стрельба из лука
  (:Pressed
    (if _isaiming
      (Default|CallPrepareShot (Variables|Default|GetElementNumber))
      (elif (Variables|Default|GetIsElementalSkill)
        _)))
  (:Released
    (if _isaiming
      (Default|CallBowShot))))

(event Input|ActionEvents|InputActionJump
  (params (Key :type Key%20Structure :default "None"))
  (bind _returnvalue (Game|GetPlayerCharacter 0))
  ;[0 1 0.08914] Прыжок
  (:Pressed
    (Character|Jump _returnvalue))
  (:Released
    (Character|StopJumping _returnvalue)))

(event Input|ActionEvents|InputActionFocusToWisp
  (params (Key :type Key%20Structure :default "None"))
  ;[0.4001 1 0.288] Фокусировка на актере-огоньке
  (:Pressed
    (Utilities|FlowControl|Gate true
      (:Exit
        ;;[0.05673 1 0.9003] Входим в режим прицела с помаркой, что это "фокус"
        (Variables|Default|SetIs%20Focused true)
        (Default|SetAimShildCameraPos (stale EventBeginPlay _asthird_person_character))
        (Utilities|FlowControl|Gate true) ; enters at Open
      )))
  (:Released
    (Utilities|FlowControl|Gate true
      (:Exit
        (Variables|Default|SetIs%20Focused false)
        (Default|SetFreeCameraPos (stale EventBeginPlay _asthird_person_character))
        (Utilities|FlowControl|Gate true) ; enters at Close
      ))))

(event Input|AxisEvents|InputAxisLookUp
  (params (AxisValue :type Float%20%28single-precision%29))
  ;[0 1 0.1072] Поворот камеры
  (Pawn|Input|AddControllerPitchInput (Game|GetPlayerCharacter 0) (* (select (Variables|Default|GetIsAiming) 0.5 1.0) AxisValue)))

(event Input|AxisEvents|InputAxisTurn
  (params (AxisValue :type Float%20%28single-precision%29))
  ;[0 1 0.1072] Поворот камеры
  (Pawn|Input|AddControllerYawInput (Game|GetPlayerCharacter 0) (* AxisValue (select (Variables|Default|GetIsAiming) 0.5 1.0))))

(event Input|AxisEvents|InputAxisMoveForward
  (params (AxisValue :type Float%20%28single-precision%29))
  ;[0 1 0.08696] Перемещение
  (Pawn|Input|AddMovementInput (Game|GetPlayerCharacter 0) (Math|Vector|GetForwardVector (Math|Rotator|MakeRotator 0.0 0.0 (.Yaw (Math|Rotator|BreakRotator (Pawn|GetControlRotation :!class /Script/Engine.Controller))))) AxisValue false))

(event Input|AxisEvents|InputAxisMoveRight
  (params (AxisValue :type Float%20%28single-precision%29))
  ;[0 1 0.08696] Перемещение
  (Pawn|Input|AddMovementInput (Game|GetPlayerCharacter 0) (Math|Vector|GetRightVector (Math|Rotator|MakeRotator 0.0 0.0 (.Yaw (Math|Rotator|BreakRotator (Pawn|GetControlRotation :!class /Script/Engine.Controller))))) AxisValue false))

(fn ConstructionScript)