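; GameInitial, with an empty Init event, saves and loads the player's element number and character transform.
; SaveGame creates a JamSaveGame if needed, fills it through the GetContollerAndPlayer helper and writes it to a slot.
; LoadGame reads that slot and applies both values to JamPlayerController and ThirdPersonCharacter.
; The slot name comes from the GameSave object's name, and LoadGame never creates that object.
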(event Custom|LoadGame
  (bind (_controller _asthird_person_character) (CallFunction|GetContollerandPlayer))
  ;[1 0.9558 0] Сохранение и загрузка
  (bind _returnvalue (SaveGame|LoadGamefromSlot (Utilities|GetObjectName (Variables|Default|GetGameSave))))
  (bind _asjam_save_game (Utilities|Casting|CastToJamSaveGame _returnvalue))
  (Variables|/Game/CodeFolder/Blueprints/Main_GG_Logic/JamPlayerController.JamPlayerController_C|SetElementNumber _controller (Variables|/Game/CodeFolder/Blueprints/Game_Logic/JamSaveGame.JamSaveGame_C|GetSaveElementalUse _asjam_save_game))
  (Transformation|SetActorTransform _asthird_person_character (Variables|/Game/CodeFolder/Blueprints/Game_Logic/JamSaveGame.JamSaveGame_C|GetSavePlayerTransform _asjam_save_game))
  (Development|PrintString "Сохранение загружено"))

(event Custom|SaveGame
  (bind (_controller _asthird_person_character) (CallFunction|GetContollerandPlayer))
  ;[1 0.9558 0] Сохранение и загрузка
  (Utilities|IsValid (Variables|Default|GetGameSave)
    (:Is%20Valid
      _)
    (:Is%20Not%20Valid
      (bind _returnvalue (SaveGame|CreateSaveGameObject "/Game/CodeFolder/Blueprints/Game_Logic/JamSaveGame.JamSaveGame_C"))
      (Variables|Default|SetGameSave _returnvalue)))
  (Variables|/Game/CodeFolder/Blueprints/Game_Logic/JamSaveGame.JamSaveGame_C|SetSaveElementalUse (Variables|Default|GetGameSave) (Variables|/Game/CodeFolder/Blueprints/Main_GG_Logic/JamPlayerController.JamPlayerController_C|GetElementNumber _controller))
  (Variables|/Game/CodeFolder/Blueprints/Game_Logic/JamSaveGame.JamSaveGame_C|SetSavePlayerTransform (Variables|Default|GetGameSave) (Transformation|GetActorTransform _asthird_person_character))
  (bind _returnvalue_2 (SaveGame|SaveGametoSlot (Variables|Default|GetGameSave) (Utilities|GetObjectName (Variables|Default|GetGameSave))))
  (if _returnvalue_2
    (Development|PrintString "Сохранение прошло успешно")
    (else
      (Development|PrintString "Сохранение не удалось"))))

(event EventInit
  ;[1 0.9434 0] Инициация настроек
)

(fn GetContollerandPlayer
  (bind _asjam_player_controller (Utilities|Casting|CastToJamPlayerController (Game|GetPlayerController 0)))
  (bind _asthird_person_character (Utilities|Casting|CastToThirdPersonCharacter (Pawn|GetControlledPawn _asjam_player_controller)))
  (return _asjam_player_controller _asthird_person_character))