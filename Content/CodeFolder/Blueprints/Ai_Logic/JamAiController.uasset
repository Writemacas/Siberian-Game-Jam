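; JamAiController is an AI controller that starts a behavior tree and exposes melee and bow attack actions.
; On BeginPlay it runs AiTree and fills Blackboard object keys: SelfActor and CanMove with the controller itself, Player with the first player character.
; MeleeAttack and BowAttack clear CanMoving, call the combo or bow shot, and print debug text.
; CanMoving is never restored here, and the melee delay leads to nothing.
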(event Custom|MeleeAttack
  (Variables|Default|SetCanMoving false)
  (Default|CallAttackCombo)
  (Development|PrintString "БЬЮ ГАВНОМ")
  (Utilities|FlowControl|Delay (Variables|Default|GetAttackDelay)))

(event Custom|BowAttack
  (Variables|Default|SetCanMoving false)
  (Default|CallBowShot)
  (Development|PrintString "КИДАЮ ГРАНААААТУ"))

(event EventBeginPlay
  (bind _blackboard (Variables|Default|GetBlackboard))
  (AI|RunBehaviorTree "/Game/CodeFolder/Blueprints/Ai_Logic/AiTree.AiTree")
  (AI|Components|Blackboard|SetValueasObject _blackboard (Utilities|Name|MakeLiteralName "SelfActor") self)
  (AI|Components|Blackboard|SetValueasObject _blackboard (Utilities|Name|MakeLiteralName "Player") (Game|GetPlayerCharacter 0))
  (AI|Components|Blackboard|SetValueasObject _blackboard (Utilities|Name|MakeLiteralName "CanMove") self))

(fn ConstructionScript)