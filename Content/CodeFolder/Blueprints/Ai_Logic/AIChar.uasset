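; AI enemy character that attacks with a bow or spear, ignores damage instigated by JamAiController and destroys itself when health drops below zero.
; AttackPlayer calls SwapWeapon to spawn and socket the weapon, then fires a delayed bow shot or sets melee combo variables.
; StunAI forwards stuns to the controller, while Ragdoll simulates physics until the character stops falling.
; ThirdPersonCharacter mark events toggle a custom-depth outline, matched by display name.
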(event Custom|SetMark_Event_0
  (params (A :type String))
  ;[0 1 0.268] Обводка персонажа при наведении
  (if (Utilities|Enum|Equal(Enum) A (Utilities|GetDisplayName self))
    (Rendering|SetRenderCustomDepth (Variables|Character|GetMesh) true)))

(event Custom|DeleteMark_Event_0
  ;[0 1 0.268] Обводка персонажа при наведении
  (Rendering|SetRenderCustomDepth (Variables|Character|GetMesh) false))

(event Custom|Ragdoll
  ;[0 1 0.268] Обводка персонажа при наведении
  (Class|SkeletalMeshComponent|SetAllBodiesSimulatePhysics (Variables|Character|GetMesh) true)
  (Utilities|FlowControl|Delay 3.0 :!label _label)
  (if (AI|Components|NavMovement|IsFalling (Variables|Character|GetCharacterMovement))
    (goto _label)
    (else
      (Class|SkeletalMeshComponent|SetAllBodiesSimulatePhysics (Variables|Character|GetMesh) false)
      (Physics|SetSimulatePhysics (Variables|Collision|GetCapsuleComponent) false))))

(event Custom|ShootAfterDelay
  ;[0.4001 1 0.288] Стрельба из лука
  (Utilities|FlowControl|Delay (Variables|CONFIG|GetShootDelaty))
  (Default|BowShot (Variables|Default|GetBowActorRef) (Transformation|GetActorForwardVector self)))

(event Game|Damage|EventAnyDamage
  (params (Damage :type Float%20%28single-precision%29) (DamageType :type Damage%20Type%20Object%20Reference) (InstigatedBy :type Controller%20Object%20Reference) (DamageCauser :type Actor%20Object%20Reference))
  (if (not (== InstigatedBy "/Game/CodeFolder/Blueprints/Ai_Logic/JamAiController.JamAiController"))
    (bind _output_get (Variables|CONFIG|SetHealtpoints (- (Variables|CONFIG|GetHealtpoints) Damage)))
    (if (< _output_get 0.0)
      (CallFunction|SwapWeapon "NewEnumerator0")
      (Actor|DestroyActor))))

(event EventBeginPlay
  ;[0 1 0.268] Обводка персонажа при наведении
  (bind _outactors (Actor|GetAllActorsOfClass "/Game/CodeFolder/Blueprints/Main_GG_Logic/ThirdPersonCharacter.ThirdPersonCharacter_C"))
  (for _array_element _outactors
    _)
  (Utilities|FlowControl|Sequence
    (:then_0
      (EventDispatchers|AssignDeleteMark _array_element (delegate Custom|DeleteMark_Event_0)))
    (:then_1
      (EventDispatchers|AssignSetMark _array_element (delegate Custom|SetMark_Event_0)))))

(fn ConstructionScript)

(fn StunAI
  (bind _asjam_ai_controller (Utilities|Casting|CastToJamAiController (Pawn|GetController)))
  (Default|CallOnStunned _asjam_ai_controller))

(fn AttackPlayer
  (params (UseWeapon :type CurrentWeapon%20Enum :default "NewEnumerator0"))
  (bind _bowactorref (Variables|Default|GetBowActorRef))
  (if (== UseWeapon (Variables|Default|GetCurrentWeaponInHand))
    _
    (else
      (CallFunction|SwapWeapon UseWeapon)))
  (switch Utilities|FlowControl|Switch|SwitchonCurrentWeapon UseWeapon
    (:NewEnumerator0
      (Development|PrintString "Standing here i realize~"))
    (:NewEnumerator1
      (Utilities|IsValid _bowactorref
        (:Is%20Valid
          (Default|PrepareforShot _bowactorref)
          (CallFunction|ShootAfterDelay))))
    (:NewEnumerator2
      (Variables|Default|SetisAttacking true)
      (Variables|Default|SetComboIndex (Math|Conversions|ToFloat(Integer) (Math|Random|RandomInteger 1)))))
  (return))

(fn SwapWeapon
  (params (New%20Weapon :type CurrentWeapon%20Enum :default "NewEnumerator0"))
  ;[0.4001 1 0.288] Освобождаем руки
  (switch Utilities|FlowControl|Switch|SwitchonCurrentWeapon (Variables|Default|GetCurrentWeaponInHand)
    (:NewEnumerator0
      _)
    (:NewEnumerator1
      ;;[0.05673 1 0.9003] Уничтожение лука
      (Actor|DestroyActor (Variables|Default|GetBowActorRef))
      (Variables|Default|SetisAiming false))
    (:NewEnumerator2
      ;;[0.05673 1 0.9003] Убираем копьё
      (Actor|DestroyActor (Variables|Default|GetSpearActorRef))))
  ;[0.4001 1 0.288] Новое оружие
  (switch Utilities|FlowControl|Switch|SwitchonCurrentWeapon New%20Weapon
    (:NewEnumerator0
      _)
    (:NewEnumerator1
      ;;[0.05673 1 0.9003] Спавн Лука
      (bind _returnvalue (Game|SpawnActorfromClass "/Game/CodeFolder/Blueprints/Main_GG_Logic/Weapon/BowActor.BowActor_C" (Math|Transform|MakeTransform "0, 0, 0" "0, 0, 0" "1,1,1") "AlwaysSpawn" 0 0))
      (bind _output_get (Variables|Default|SetBowActorRef _returnvalue))
      (Transformation|AttachComponentToComponent _output_get (Variables|Character|GetMesh) (Variables|CONFIG|GetLeftHandSocketName) "SnapToTarget" "SnapToTarget" "KeepWorld" true)
      (Variables|Default|SetisAiming true))
    (:NewEnumerator2
      ;;[0.05673 1 0.9003] Спавним копьё
      (bind _returnvalue_2 (Game|SpawnActorfromClass "/Game/CodeFolder/Blueprints/Main_GG_Logic/Weapon/SpearActor.SpearActor_C" (Math|Transform|MakeTransform "0, 0, 0" "0, 0, 0" "1,1,1") "AlwaysSpawn" 0 0))
      (bind _output_get_2 (Variables|Default|SetSpearActorRef _returnvalue_2))
      (Transformation|AttachComponentToComponent _output_get_2 (Variables|Character|GetMesh) (Variables|CONFIG|GetLeftHandSocketName) "SnapToTarget" "SnapToTarget" "KeepWorld" true)))
  (Variables|Default|SetCurrentWeaponInHand New%20Weapon)
  (return))