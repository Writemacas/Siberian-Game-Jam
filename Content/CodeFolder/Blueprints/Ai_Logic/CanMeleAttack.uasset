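; Behavior Tree service that decides whether the AI is close enough to the player for a melee attack.
; On activation, it measures the distance between the Player and SelfActor Blackboard actors and compares it to the MeleRange key.
; It writes the result to CanMeleAttackBool, true when the player is within or at that range.
; The check runs only on activation, with no tick update.
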(event EventReceiveActivation
  (params (OwnerActor :type Actor%20Object%20Reference))
  (Class|BTFunctionLibrary|SetBlackboardValueasBool (Variables|Default|GetCanMeleAttackBool) (>= (Class|BTFunctionLibrary|GetBlackboardValueasFloat (Variables|Default|GetMeleRange)) (Math|Vector|Distance(Vector) (Transformation|GetActorLocation (AI|BehaviorTree|GetBlackboardValueasActor (Variables|Default|GetPlayer))) (Transformation|GetActorLocation (AI|BehaviorTree|GetBlackboardValueasActor (Variables|Default|GetSelfActor)))))))