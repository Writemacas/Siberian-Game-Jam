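; Behavior tree service that decides whether the AI has a clear line of fire to the player.
; On activation, it traces from the player to the AI against world, pawn and destructible objects, ignoring both actors.
; It writes CanShootBool to the blackboard as true when nothing blocks the trace.
; The check does not repeat on tick, and the trace draws a one-frame debug line.
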(event EventReceiveActivation
  (params (OwnerActor :type Actor%20Object%20Reference))
  (bind _player (Variables|Default|GetPlayer))
  (bind _selfactor (Variables|Default|GetSelfActor))
  (bind _returnvalue (AI|BehaviorTree|GetBlackboardValueasActor _selfactor))
  (bind _returnvalue_2 (AI|BehaviorTree|GetBlackboardValueasActor _player))
  (bind _returnvalue_3 (Collision|LineTraceForObjects (Transformation|GetActorLocation _returnvalue_2) (Transformation|GetActorLocation _returnvalue) (Utilities|Array|MakeArray "ObjectTypeQuery1" "ObjectTypeQuery2" "ObjectTypeQuery3" "ObjectTypeQuery6") false (Utilities|Array|MakeArray _returnvalue_2 _returnvalue) "ForOneFrame"))
  (Class|BTFunctionLibrary|SetBlackboardValueasBool (Variables|Default|GetCanShootBool) (not _returnvalue_3)))