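; Base logic listener object that reacts to activation signals from actors carrying the tag it listens to.
; On BeginPlay it finds all actors with that tag and binds its activation and deactivation handlers to interactable objects' events.
; Player-only triggers that participate in logic map enter and exit to the same handlers.
; Both handlers are empty here.
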(event Custom|HeardActivationSignal)

(event Custom|HeardDeactivationSignal)

(event EventBeginPlay
  (bind _outactors (Actor|GetAllActorswithTag (Utilities|String|StringToName (Variables|Default|GetTag%20To%20Listen))))
  (for _array_element _outactors
    (bind _aspar_interactable_object (Utilities|Casting|CastToPAR_InteractableObject _array_element)
      (:then
        (EventDispatchers|BindEventtoOnActivated _aspar_interactable_object (delegate Custom|HeardActivationSignal))
        (EventDispatchers|BindEventtoOnDeactivated _aspar_interactable_object (delegate Custom|HeardDeactivationSignal)))
      (:CastFailed
        (bind _astrigger_player_body_only (Utilities|Casting|CastToTriggerPlayerBodyOnly _array_element))
        (if (Variables|/Game/CodeFolder/utillity/TriggerPlayerBodyOnly.TriggerPlayerBodyOnly_C|GetParticipateInLogic _astrigger_player_body_only)
          (EventDispatchers|BindEventtoEventPlayerEnteredTrigger _astrigger_player_body_only (delegate Custom|HeardActivationSignal))
          (EventDispatchers|BindEventtoEventPlayerExitedTrigger _astrigger_player_body_only (delegate Custom|HeardDeactivationSignal)))))))

(fn ConstructionScript)