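; Logic object, such as a torch, that arrow projectile hits switch on or off, marked as a temporary solution.
; TriggerMode allows activation, deactivation or both, matching arrow tags against activating and deactivating type tags.
; State changes fire CallOnActivated or CallOnDeactivated once and show or hide the effects component.
; BeginPlay sets state and effects without those calls, starting lit only in Deactivate Only mode.
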(event EventBeginPlay
  (bind _onactivatedeffects (Variables|Default|GetOnActivatedEffects))
  ;[0.4124 1 0.2916] Изначально зажигаем элемент, если его надо тушить
  (if (== (Variables|Default|GetTriggerMode) (Utilities|Enum|LiteralenumElementTriggerMode "NewEnumerator1"))
    ;[0.5587 1 0.2568] Включаем видимость "огня" при включенном факеле и наоборот
    (Variables|Default|SetIsStartActivated true)
    (Rendering|SetVisibility _onactivatedeffects true true)
    (else
      (Variables|Default|SetIsStartActivated false)
      (Rendering|SetVisibility _onactivatedeffects false true))))

(event Collision|EventHit
  (params (MyComp :type Primitive%20Component%20Object%20Reference) (Other :type Actor%20Object%20Reference) (OtherComp :type Primitive%20Component%20Object%20Reference) (bSelfMoved :type Boolean) (HitLocation :type Vector :default "0, 0, 0") (HitNormal :type Vector :default "0, 0, 0") (NormalImpulse :type Vector :default "0, 0, 0") (Hit :type Hit%20Result%20Structure%20%28by%20ref%29))
  (bind _onactivatedeffects (Variables|Default|GetOnActivatedEffects))
  ;[0.5725 0.6653 1] Пересечение со стрелой (Временное решение)
  (bind _asarrow_projetile (Utilities|Casting|CastToArrowProjetile Other))
  (switch Utilities|FlowControl|Switch|SwitchonElementTriggerMode (Variables|Default|GetTriggerMode)
    (:NewEnumerator0
      (if (Actor|ActorHasTag _asarrow_projetile (Variables|Default|GetActivatingTypeTag))
        ;;[0.1955 0.3473 1] Исключаем повторное срабатывание события
        (if (not (Variables|Default|GetIsStartActivated)) :!label _label
          (Default|CallOnActivated)
          ;[0.5587 1 0.2568] Включаем видимость "огня" при включенном факеле и наоборот
          (Variables|Default|SetIsStartActivated true)
          (Rendering|SetVisibility _onactivatedeffects true true))))
    (:NewEnumerator1
      (if (Actor|ActorHasTag _asarrow_projetile (Variables|Default|GetDeactivatingTypeTag))
        (if (Variables|Default|GetIsStartActivated) :!label _label_2
          (Default|CallOnDeactivated)
          (Variables|Default|SetIsStartActivated false)
          (Rendering|SetVisibility _onactivatedeffects false true))))
    (:NewEnumerator2
      (if (or (Actor|ActorHasTag _asarrow_projetile (Variables|Default|GetActivatingTypeTag)) (Actor|ActorHasTag _asarrow_projetile (Variables|Default|GetDeactivatingTypeTag)))
        (if (Actor|ActorHasTag _asarrow_projetile (Variables|Default|GetActivatingTypeTag))
          (goto _label)
          (else
            (goto _label_2)))))))

(fn ConstructionScript)